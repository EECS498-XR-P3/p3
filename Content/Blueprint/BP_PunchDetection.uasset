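; BP_PunchDetection is a zone actor that decides whether the VR player's punches count as valid.
; Each Tick it follows the VRPawn's head position at a fixed offset, without using head rotation.
; It sets IsPunchValid on the pawn while both left and right in-zone flags are true, clearing it after a timeout otherwise.
; The Box overlap handler only casts, and nothing here sets those flags.
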(event OnComponentBeginOverlap(Box)
  (params (OverlappedComponent :type Primitive%20Component%20Object%20Reference) (OtherActor :type Actor%20Object%20Reference) (OtherComp :type Primitive%20Component%20Object%20Reference) (OtherBodyIndex :type Integer) (bFromSweep :type Boolean) (SweepResult :type Hit%20Result%20Structure%20%28by%20ref%29))
  (bind _asvrpawn (Utilities|Casting|CastToVRPawn OtherActor))
  (Utilities|IsValid _asvrpawn))

(event EventBeginPlay
  (Rendering|SetVisibility (Variables|Debug|GetStaticMeshComponent) true false)
  (bind _asvrpawn (Utilities|Casting|CastToVRPawn (Game|Player|GetPlayerPawn 0)))
  (Utilities|IsValid _asvrpawn
    (:Is%20Valid
      (Variables|Default|SetVRPawn _asvrpawn))))

(event Collision|EventActorBeginOverlap
  (params (OtherActor :type Actor%20Object%20Reference)))

(event EventTick
  (params (DeltaSeconds :type Float%20%28single-precision%29))
  (Transformation|SetActorLocationAndRotation (+ (Variables|/Game/VRTemplate/Blueprints/VRPawn.VRPawn_C|GetHeadPos (Variables|Default|GetVRPawn)) "20.000000,-50.000000,-50.000000") (Math|Rotator|MakeRotator 0.0 0.0 0.0))
  (if (and (Variables|Default|GetLeftInDetectZone) (Variables|Default|GetRightInDetectZone))
    (Variables|Default|SettimeElapse 0.0)
    (Variables|/Game/VRTemplate/Blueprints/VRPawn.VRPawn_C|SetisPunchValid (Variables|Default|GetVRPawn) true)
    (else
      (bind _output_get (Variables|Default|SettimeElapse (+ DeltaSeconds (Variables|Default|GettimeElapse))))
      (if (>= _output_get (Variables|Default|GettimeToDisablePunch))
        (Variables|/Game/VRTemplate/Blueprints/VRPawn.VRPawn_C|SetisPunchValid (Variables|Default|GetVRPawn) false)))))

(fn ConstructionScript)