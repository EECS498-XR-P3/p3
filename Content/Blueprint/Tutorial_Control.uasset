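; Tutorial controller for a VR boxing game that walks the player through dodging, posture, punching back attacks and pausing.
; Tick runs an enum state machine that loads each message into TutorialPopup and queues the next state.
; Each message pauses the game until the popup's Interacted flag unpauses it and allows the next.
; Setting the final message also turns off the VRPawn's interact ray and debug-prints that flag.
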(event Collision|EventActorBeginOverlap
  (params (OtherActor :type Actor%20Object%20Reference)))

(event EventTick
  (params (DeltaSeconds :type Float%20%28single-precision%29))
  (if (Variables|Default|GetTextSet)
    (if (Variables|Default|GetDisplayed)
      (if (Variables|/Game/Blueprint/UI/BP_Popup.BP_Popup_C|GetInteracted (Variables|Default|GetTutorial_Popup))
        (Game|SetGamePaused false)
        (Variables|Default|SetDisplayed false)
        (Variables|Default|SetTextSet false))
      (else
        (Game|SetGamePaused true)
        (Variables|Default|SetDisplayed true)))
    (else
      (switch Utilities|FlowControl|Switch|SwitchonTutorialStates (Variables|Default|GetCurrentState)
        (:NewEnumerator0
          (Default|Reset (Variables|Default|GetTutorial_Popup) "Welcome to the tutorial! You will learn how to dodge enemies' attack and fight back here.")
          (Variables|Default|SetCurrentState "NewEnumerator1")
          (Variables|Default|SetTextSet true :!label _label)
          (Utilities|FlowControl|DelayUntilNextTick))
        (:NewEnumerator1
          (Default|Reset (Variables|Default|GetTutorial_Popup) "Squat down to dodge sticks!")
          (Variables|Default|SetCurrentState "NewEnumerator2")
          (goto _label))
        (:NewEnumerator2
          (Default|Reset (Variables|Default|GetTutorial_Popup) "You may punch some of the enemy attacks back to deal damage to the enemy. First, you have to have a right boxing posture! Keep both of your hands in front of you in the reset zone. If any of your hands leaves the reset zone and it turns red, you will not able to hit back attacks!")
          (Variables|Default|SetCurrentState "NewEnumerator3")
          (goto _label))
        (:NewEnumerator3
          (Default|Reset (Variables|Default|GetTutorial_Popup) "You have a fire left fist and a ice right fist. Hit fire balls back with your left fist and hit ice balls back with your right fist. There are two types of attacks that you can fight back: jab and hook. Jab attacks have a shattered glass icon on the balls and hook attacks have arrows pointinng the direction where you show perform a hook.")
          (Variables|Default|SetCurrentState "NewEnumerator4")
          (goto _label))
        (:NewEnumerator4
          (Default|Reset (Variables|Default|GetTutorial_Popup) "This is the end of the tutorial. You may press both triggers to pause the game. Good luck and have fun!")
          (Variables|Default|SetCurrentState "NewEnumerator5")
          (Variables|Default|SetTextSet true)
          (bind _asvrpawn (Utilities|Casting|CastToVRPawn (Game|Player|GetPlayerPawn 0)))
          (bind _output_get (Variables|/Game/VRTemplate/Blueprints/VRPawn.VRPawn_C|SetDrawInteractRay _asvrpawn false))
          (Development|PrintString (Utilities|String|ToString(Boolean) _output_get) true true "(R=0.000000,G=0.660000,B=1.000000,A=1.000000)" 1.2e+02))))))

(fn ConstructionScript)