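; Dodge_Attack is an actor that travels forward as a thin, elongated shape, apparently an attack to be dodged.
; Each tick it offsets itself along its forward vector by Speed, without sweep or DeltaSeconds scaling, and reapplies a fixed scale.
; The self-destroy check compares two constants and is always false, so it never fires.
; It has no active overlap or damage logic.
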(event Collision|EventActorBeginOverlap
  (params (OtherActor :type Actor%20Object%20Reference))
  (|CallParentFunction OtherActor) ; This node is disabled and will not be called.\nDrag off pins to build functionality.
)

(event EventTick
  (params (DeltaSeconds :type Float%20%28single-precision%29))
  (|CallParentFunction DeltaSeconds)
  (Class|Actor|AddActorWorldTransform (Math|Conversions|ToTransform(Vector) (* (Transformation|GetActorForwardVector) (Variables|Default|GetSpeed))) false false)
  (Transformation|SetActorScale3D "0.200000,5.000000,0.010000")
  (if (>= 0.0 8.0)
    (Actor|DestroyActor)))

(fn ConstructionScript
  (|CallParentFunction))