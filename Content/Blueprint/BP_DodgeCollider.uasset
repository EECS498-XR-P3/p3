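; BP_DodgeCollider is an invisible collider that follows the VR player's head and destroys BP_DeflectOrDestroy actors that touch it.
; Each Tick it reads HeadPos from the VRPawn and moves itself there with a fixed offset; head rotation is not applied.
; When its Box overlaps one of those actors, it destroys that actor and plays a swinging axe sound in 2D.
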(event OnComponentBeginOverlap(Box)
  (params (OverlappedComponent :type Primitive%20Component%20Object%20Reference) (OtherActor :type Actor%20Object%20Reference) (OtherComp :type Primitive%20Component%20Object%20Reference) (OtherBodyIndex :type Integer) (bFromSweep :type Boolean) (SweepResult :type Hit%20Result%20Structure%20%28by%20ref%29))
  (bind _asbp_deflect_or_destroy (Utilities|Casting|CastToBP_DeflectOrDestroy OtherActor))
  (Utilities|IsValid _asbp_deflect_or_destroy
    (:Is%20Valid
      (Actor|DestroyActor OtherActor)
      (Audio|PlaySound2D "/Game/sfx/514162__zhr__swinging-axe.514162__zhr__swinging-axe" 6.0 1.0 0.0 0 0))))

(event EventBeginPlay
  (Rendering|SetVisibility (Variables|Debug|GetStaticMeshComponent) false false))

(event Collision|EventActorBeginOverlap
  (params (OtherActor :type Actor%20Object%20Reference)))

(event EventTick
  (params (DeltaSeconds :type Float%20%28single-precision%29))
  (bind _asvrpawn (Utilities|Casting|CastToVRPawn (Game|Player|GetPlayerPawn 0)))
  (Utilities|IsValid _asvrpawn
    (:Is%20Valid
      (Transformation|SetActorLocationAndRotation (+ (Variables|/Game/VRTemplate/Blueprints/VRPawn.VRPawn_C|GetHeadPos _asvrpawn) "-50.000000,-400.000000,-200.000000") (Math|Rotator|MakeRotator 0.0 0.0 0.0)))))

(fn ConstructionScript)