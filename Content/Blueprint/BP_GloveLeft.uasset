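; BP_GloveLeft is the left VR glove actor, which follows the player's left controller and handles punch contact.
; Every tick it copies the VRPawn's left controller position and rotation and stores the controller velocity.
; Its capsule overlaps toggle the left in-zone flag on BP_PunchDetection actors.
; When the pawn's punch is valid, a hit on a BP_DeflectOrDestroy triggers deflect-or-destroy with impact location and velocity.
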(event OnComponentBeginOverlap(Capsule)
  (params (OverlappedComponent :type Primitive%20Component%20Object%20Reference) (OtherActor :type Actor%20Object%20Reference) (OtherComp :type Primitive%20Component%20Object%20Reference) (OtherBodyIndex :type Integer) (bFromSweep :type Boolean) (SweepResult :type Hit%20Result%20Structure%20%28by%20ref%29))
  (bind _asbp_punch_detection (Utilities|Casting|CastToBP_PunchDetection OtherActor)
    (:then
      (Utilities|IsValid _asbp_punch_detection
        (:Is%20Valid
          (Variables|/Game/Blueprint/BP_PunchDetection.BP_PunchDetection_C|SetLeftInDetectZone _asbp_punch_detection true))
        (:Is%20Not%20Valid
          _)))
    (:CastFailed
      _))
  (if (Variables|/Game/VRTemplate/Blueprints/VRPawn.VRPawn_C|GetisPunchValid (Variables|Default|GetVRPawn))
    (bind _asbp_deflect_or_destroy (Utilities|Casting|CastToBP_DeflectOrDestroy OtherActor))
    (Utilities|IsValid _asbp_deflect_or_destroy
      (:Is%20Valid
        (Default|DeflectorDestroy _asbp_deflect_or_destroy (.Location (Collision|BreakHitResult SweepResult)) true (Variables|Default|Getvelocity))))))

(event OnComponentEndOverlap(Capsule)
  (params (OverlappedComponent :type Primitive%20Component%20Object%20Reference) (OtherActor :type Actor%20Object%20Reference) (OtherComp :type Primitive%20Component%20Object%20Reference) (OtherBodyIndex :type Integer))
  (bind _asbp_punch_detection (Utilities|Casting|CastToBP_PunchDetection OtherActor))
  (Utilities|IsValid _asbp_punch_detection
    (:Is%20Valid
      (Variables|/Game/Blueprint/BP_PunchDetection.BP_PunchDetection_C|SetLeftInDetectZone _asbp_punch_detection false))))

(event EventBeginPlay
  (bind _asvrpawn (Utilities|Casting|CastToVRPawn (Game|Player|GetPlayerPawn 0)))
  (Utilities|IsValid _asvrpawn
    (:Is%20Valid
      (Variables|Default|SetVRPawn _asvrpawn))))

(event Collision|EventActorBeginOverlap
  (params (OtherActor :type Actor%20Object%20Reference)))

(event EventTick
  (params (DeltaSeconds :type Float%20%28single-precision%29))
  (bind _vrpawn (Variables|Default|GetVRPawn))
  (Transformation|SetActorLocationAndRotation (Variables|/Game/VRTemplate/Blueprints/VRPawn.VRPawn_C|GetLeftControllerPos _vrpawn) (Variables|/Game/VRTemplate/Blueprints/VRPawn.VRPawn_C|GetLeftControllerRot _vrpawn))
  (Variables|Default|Setvelocity (Variables|/Game/VRTemplate/Blueprints/VRPawn.VRPawn_C|GetLeftControllerVelocity (Variables|Default|GetVRPawn))))

(fn ConstructionScript)