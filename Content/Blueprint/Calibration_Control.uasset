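; VR calibration controller that measures the player's arm length and squat depth for punch and dodge sensing, starting at BeginPlay.
; A Tick-driven state machine shows each instruction popup, pauses the game, then advances once the popup is interacted with.
; It stores the averaged world-X controller offset from the pawn and the pawn's Z drop in the Instance_Data game instance.
; The menu stays hidden until calibration finishes.
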(event EventBeginPlay
  (CallFunction|BeginCalibration))

(event Collision|EventActorBeginOverlap
  (params (OtherActor :type Actor%20Object%20Reference)))

(event EventTick
  (params (DeltaSeconds :type Float%20%28single-precision%29))
  (if (Variables|Default|GetCalibrating)
    (if (Variables|Default|GetTextSet)
      (if (Variables|Default|GetDisplayed)
        (if (Variables|/Game/Blueprint/UI/BP_Calibration_Popup.BP_Calibration_Popup_C|GetInteracted (Variables|Default|GetCalibration%20Popup))
          (Game|SetGamePaused false)
          (Variables|Default|SetDisplayed false)
          (Variables|Default|SetTextSet false))
        (else
          (Game|SetGamePaused true)
          (Variables|Default|SetDisplayed true)))
      (else
        (switch Utilities|FlowControl|Switch|SwitchonCalibrationStates (Variables|Default|GetCurrentState)
          (:NewEnumerator0
            (Default|Reset (Variables|Default|GetCalibration%20Popup) "Calibration: 
 
Before you can play, we must measure your arm length and squat distance so we can correctly sense your punches and dodges. Press both triggers to begin. ")
            (Variables|Default|SetCurrentState "NewEnumerator1")
            (Variables|Default|SetTextSet true :!label _label)
            (Utilities|FlowControl|DelayUntilNextTick))
          (:NewEnumerator1
            (Default|Reset (Variables|Default|GetCalibration%20Popup) "Calibrate Punch Length: 
 
Hold out your arms straight in front of you. When you are ready, press both triggers simultaneously to capture your arm length.")
            (Variables|Default|SetCurrentState "NewEnumerator2")
            (goto _label))
          (:NewEnumerator2
            (bind _asinstance_data (Utilities|Casting|CastToInstance_Data (Game|GetGameInstance)))
            (bind _asvrpawn (Utilities|Casting|CastToVRPawn (Game|Player|GetPlayerPawn 0)))
            (Variables|/Game/Scripts/Instance_Data.Instance_Data_C|SetArm_Length _asinstance_data (/ (+ (- (.X (Class|KismetMathLibrary|BreakVector3f (.Location (Math|Transform|BreakTransform (Transformation|GetWorldTransform (Variables|/Game/VRTemplate/Blueprints/VRPawn.VRPawn_C|GetMotionControllerLeft _asvrpawn)))))) (.X (Class|KismetMathLibrary|BreakVector3f (.Location (Math|Transform|BreakTransform (Transformation|GetActorTransform _asvrpawn)))))) (- (.X (Class|KismetMathLibrary|BreakVector3f (.Location (Math|Transform|BreakTransform (Transformation|GetWorldTransform (Variables|/Game/VRTemplate/Blueprints/VRPawn.VRPawn_C|GetMotionControllerRight _asvrpawn)))))) (.X (Class|KismetMathLibrary|BreakVector3f (.Location (Math|Transform|BreakTransform (Transformation|GetActorTransform _asvrpawn))))))) 2.0))
            (Variables|Default|SetheadStartZ (.Z (Class|KismetMathLibrary|BreakVector3f (.Location (Math|Transform|BreakTransform (Transformation|GetActorTransform _asvrpawn))))))
            (Default|Reset (Variables|Default|GetCalibration%20Popup) "Calibrate Squat Depth: 
 
Perform the beginning of a squat, stopping at the movement's lowest point. While there, press both triggers simultaneously to capture your squat depth.")
            (Variables|Default|SetCurrentState "NewEnumerator3")
            (goto _label))
          (:NewEnumerator3
            (bind _asinstance_data_2 (Utilities|Casting|CastToInstance_Data (Game|GetGameInstance)))
            (bind _asvrpawn_2 (Utilities|Casting|CastToVRPawn (Game|Player|GetPlayerPawn 0)))
            (Variables|/Game/Scripts/Instance_Data.Instance_Data_C|SetSquatDepth _asinstance_data_2 (- (Variables|Default|GetheadStartZ) (.Z (Class|KismetMathLibrary|BreakVector3f (.Location (Math|Transform|BreakTransform (Transformation|GetActorTransform _asvrpawn_2)))))))
            (Variables|Default|SetCalibrating false)))))
    (else
      (Rendering|SetVisibility (Variables|/Script/Engine.Actor|GetRootComponent (Variables|Default|GetCalibration%20Popup)) false true)
      (Rendering|SetVisibility (Variables|/Script/Engine.Actor|GetRootComponent (Variables|Default|GetMenu)) true true))))

(fn ConstructionScript)

(fn BeginCalibration
  (Rendering|SetVisibility (Variables|/Script/Engine.Actor|GetRootComponent (Variables|Default|GetCalibration%20Popup)) true true)
  (Variables|Default|SetCalibrating true)
  (Rendering|SetVisibility (Variables|/Script/Engine.Actor|GetRootComponent (Variables|Default|GetMenu)) false true))