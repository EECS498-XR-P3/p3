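; Right_Hooks is a VR punch-target projectile that flies forward until the player deflects it or it is destroyed.
; DeflectOrDestroy checks the punching hand against the attack type and classifies hit direction from velocity, then either deflects with haptics and scoring or hits the VRPawn and destroys itself.
; Tick reverses deflected motion at double speed with a Y drift that flips past a computed X midpoint.
; The attack-type material setters are disconnected, and the Tick timeout never fires.
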(event EventBeginPlay
  (|CallParentFunction)
  (Variables|Default|SetnegativeSpeed (* (Variables|Default|Getspeed) -1.0))
  (Variables|Default|SetnegativeDelta (* (Variables|Default|Getdelta) -1.0))
  (bind _returnvalue (Actor|GetActorOfClass "/Game/Blueprint/BP_EnemySpawnPointForCalc.BP_EnemySpawnPointForCalc_C"))
  (Variables|Default|SetenemySpawnPoint (Transformation|GetWorldLocation (Variables|/Script/Engine.Actor|GetRootComponent _returnvalue)))
  (switch Utilities|FlowControl|Switch|SwitchonAttackType (Variables|Default|GetattackType)
    (:NewEnumerator0
      (CallFunction|SetLeftAttack))
    (:NewEnumerator1
      (CallFunction|SetRightAttack))
    (:NewEnumerator2
      (CallFunction|SetMixedAttack))))

(event Collision|EventActorBeginOverlap
  (params (OtherActor :type Actor%20Object%20Reference))
  (|CallParentFunction OtherActor) ; This node is disabled and will not be called.\nDrag off pins to build functionality.
)

(event EventTick
  (params (DeltaSeconds :type Float%20%28single-precision%29))
  (bind _returnvalue (Transformation|GetActorForwardVector))
  (bind _speed (Variables|Default|Getspeed))
  (bind _staticmeshcomponent (Variables|Default|GetStaticMeshComponent))
  (bind _returnvalue_2 (Transformation|GetWorldLocation _staticmeshcomponent))
  (bind _returnvalue_3 (* _speed -2.0))
  (bind _returnvalue_4 (* _returnvalue _returnvalue_3))
  (|CallParentFunction DeltaSeconds)
  (if (Variables|Default|GetisDestroying)
    (Actor|DestroyActor)
    (elif (Variables|Default|GetisDeflecting)
      (if (> (.x _returnvalue_2) (Variables|Default|GetmidXPoint))
        (if (> (.x _returnvalue_2) (.x (Variables|Default|GetenemySpawnPoint)))
          _
          (else
            (Variables|Default|Setdelta (Variables|Default|GetnegativeDelta)))))
      (Class|Actor|AddActorWorldTransform (Math|Conversions|ToTransform(Vector) (Math|Vector|MakeVector (.x _returnvalue_4) (- (.y _returnvalue_4) (Variables|Default|Getdelta)) (.z _returnvalue_4))) false false)
      (if (>= 0.0 8.0)
        (Actor|DestroyActor))
      (else
        (Class|Actor|AddActorWorldTransform (Math|Conversions|ToTransform(Vector) (* (Transformation|GetActorForwardVector) (Variables|Default|GetSpeed))) false false)
        (if (>= 0.0 8.0)
          (Actor|DestroyActor))))))

(fn ConstructionScript
  (|CallParentFunction))

(fn SetMixedAttack)

(fn SetLeftAttack)

(fn SetRightAttack)

(fn DeflectorDestroy
  (params (Impact%20Location :type Vector :default "0, 0, 0") (isLeftHit :type Boolean) (velocity :type Vector :default "0, 0, 0"))
  (bind _returnvalue (Game|GetPlayerController 0))
  (|CallParentFunction Impact%20Location isLeftHit velocity)
  (Variables|Default|SethitVelocity velocity)
  (if (Variables|Default|GetisDestroy)
    (Variables|Default|SetisDestroying true)
    (elif isLeftHit
      (if (Utilities|Enum|NotEqual(Enum) (Variables|Default|GetattackType) "NewEnumerator1")
        (if (<= (.x (Variables|Default|GethitVelocity)) -2e+01) :!label _label
          (Variables|Default|SetreceivedAttack "NewEnumerator0")
          (bind _output_get (Variables|Default|SetgetHitPos (Transformation|GetWorldLocation (Variables|Default|GetStaticMeshComponent)) :!label _label_2))
          (Variables|Default|SetmidXPoint (/ (- (.x (Variables|Default|GetenemySpawnPoint)) (.x _output_get)) 2.0))
          (Variables|Default|SetisDeflecting true)
          (if isLeftHit
            (Class|PlayerController|PlayHapticEffect _returnvalue "/Game/Haptic/Short_rumble.Short_rumble" "Left" 1.0 false)
            (else
              (Class|PlayerController|PlayHapticEffect _returnvalue "/Game/Haptic/Short_rumble.Short_rumble" "Right" 1.0 false)))
          (bind _asbp_deflect_or_destroy (Utilities|Casting|CastToBP_DeflectOrDestroy (Actor|GetParentActor)))
          (Default|SetCount (Variables|Default|GetScoreComponent) (+ (Variables|/Game/UI/WBP_ScoreCount.WBP_ScoreCount_C|GetCount (Variables|/Game/Blueprint/BP_DeflectOrDestroy.BP_DeflectOrDestroy_C|GetScoreComponent _asbp_deflect_or_destroy)) 1))
          (Default|IncPunches (Variables|/Game/Blueprint/BP_DeflectOrDestroy.BP_DeflectOrDestroy_C|GetPauseComponent _asbp_deflect_or_destroy))
          (elif (>= (.y (Variables|Default|GethitVelocity)) 2e+01)
            (Variables|Default|SetreceivedAttack "NewEnumerator1")
            (goto _label_2)
            (elif (<= (.y (Variables|Default|GethitVelocity)) -2e+01)
              (Variables|Default|SetreceivedAttack "NewEnumerator3")
              (goto _label_2)
              (elif (>= (.z (Variables|Default|GethitVelocity)) 2e+01)
                (Variables|Default|SetreceivedAttack "NewEnumerator2")
                (goto _label_2)
                (else
                  (bind _asvrpawn (Utilities|Casting|CastToVRPawn (Game|Player|GetPlayerPawn 0) :!label _label_3))
                  (Default|Hit _asvrpawn)
                  (Variables|Default|SetisDestroying true))))))
        (else
          (goto _label_3)))
      (elif (Utilities|Enum|NotEqual(Enum) (Variables|Default|GetattackType) "NewEnumerator0")
        (goto _label)
        (else
          (goto _label_3))))))