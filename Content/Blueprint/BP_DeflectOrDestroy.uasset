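; BP_DeflectOrDestroy is an actor that, when triggered, either gets pushed away from the player or destroys itself.
; DeflectOrDestroy stores the impact location and uses IsDestroy to set the destroying or deflecting state, with a leftover debug print when deflecting.
; Tick moves a deflecting actor along the player-to-actor vector, scaled by delta time, or destroys it.
; DetermineJabAttack, uncalled here, can cancel deflection based on hit side and the owner's Jab_Attacks type.
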(event EventBeginPlay)

(event Collision|EventActorBeginOverlap
  (params (OtherActor :type Actor%20Object%20Reference)))

(event EventTick
  (params (DeltaSeconds :type Float%20%28single-precision%29))
  (bind _returnvalue (Transformation|GetActorLocation))
  (if (Variables|Default|GetisDeflecting)
    ;[1 1 1] Deflect
    (Transformation|SetActorLocation (+ (* (- _returnvalue (Transformation|GetActorLocation (Game|Player|GetPlayerPawn 0))) DeltaSeconds) _returnvalue) false false)
    (elif (Variables|Default|GetisDestroying)
      ;[1 1 1] Destroy
      (Actor|DestroyActor))))

(fn ConstructionScript)

(fn DeflectorDestroy
  (params (Impact%20Location :type Vector) (isLeftHit :type Boolean))
  (Variables|Default|SetImpactLocation Impact%20Location)
  (if (Variables|Default|GetisDestroy)
    (Variables|Default|SetisDestroying true)
    (else
      (Variables|Default|SetisDeflecting true)
      (Development|PrintString "I am in the wrong place lo wut am I doing" true true "(R=0.000000,G=0.660000,B=1.000000,A=1.000000)" 6e+01))))

(fn DetermineJabAttack
  (params (isLeftHit :type Boolean))
  (bind _asjab_attacks (Utilities|Casting|CastToJab_Attacks (Components|GetOwner)))
  (Utilities|IsValid _asjab_attacks
    (:Is%20Valid
      (if isLeftHit
        (if (Utilities|Enum|Equal(Enum) (Variables|/Game/Blueprint/Jab_Attacks.Jab_Attacks_C|GetattackType _asjab_attacks) "NewEnumerator1")
          (Variables|Default|SetisDeflecting false))
        (elif (Utilities|Enum|Equal(Enum) (Variables|/Game/Blueprint/Jab_Attacks.Jab_Attacks_C|GetattackType _asjab_attacks) "NewEnumerator0")
          (Variables|Default|SetisDeflecting false))))))