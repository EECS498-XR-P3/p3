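; Pause_Menu_Control is an actor that opens the VR pause menu and pauses the game.
; It hides the referenced PauseMenu actor and disables its collision on BeginPlay.
; Each Tick it polls the player VRPawn, and when both triggers are held it shows the menu with collision, turns on the pawn's interact ray and pauses the game.
; This Blueprint has no logic to close the menu or unpause.
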(event EventBeginPlay
  (bind _pause_menu (Variables|Default|GetPause_Menu))
  (Rendering|SetActorHiddenInGame _pause_menu true)
  (Collision|SetActorEnableCollision _pause_menu false))

(event Collision|EventActorBeginOverlap
  (params (OtherActor :type Actor%20Object%20Reference)))

(event EventTick
  (params (DeltaSeconds :type Float%20%28single-precision%29))
  (bind _pause_menu (Variables|Default|GetPause_Menu))
  (bind _asvrpawn (Utilities|Casting|CastToVRPawn (Game|Player|GetPlayerPawn 0)))
  (if (and (Variables|/Game/VRTemplate/Blueprints/VRPawn.VRPawn_C|GetleftTriggerHeld _asvrpawn) (Variables|/Game/VRTemplate/Blueprints/VRPawn.VRPawn_C|GetrightTriggerHeld _asvrpawn))
    (Rendering|SetActorHiddenInGame _pause_menu false)
    (Collision|SetActorEnableCollision _pause_menu true)
    (bind _asvrpawn_2 (Utilities|Casting|CastToVRPawn (Game|Player|GetPlayerPawn 0)))
    (Variables|/Game/VRTemplate/Blueprints/VRPawn.VRPawn_C|SetDrawInteractRay_0 _asvrpawn_2 true)
    (Game|SetGamePaused true)))

(fn ConstructionScript)