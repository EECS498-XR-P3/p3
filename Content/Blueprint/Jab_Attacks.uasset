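; Jab attack projectile for a VR game, deflected by hitting it with the matching hand.
; BeginPlay sets a left, right or mixed material from AttackType, and Tick moves the actor forward by Speed.
; DeflectOrDestroy extends the parent: a valid hand reverses travel, while a wrong hand calls Hit on the VRPawn and flags destruction for Tick.
; Mixed attacks accept either hand; Tick's timeout branch compares constants, so never fires.
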(event EventBeginPlay
  (|CallParentFunction)
  (Variables|Default|SetnegativeSpeed (* (Variables|Default|Getspeed) -1.0))
  (switch Utilities|FlowControl|Switch|SwitchonAttackType (Variables|Default|GetattackType)
    (:NewEnumerator0
      (CallFunction|SetLeftAttack))
    (:NewEnumerator1
      (CallFunction|SetRightAttack))
    (:NewEnumerator2
      (CallFunction|SetMixedAttack))))

(event Collision|EventActorBeginOverlap
  (params (OtherActor :type Actor%20Object%20Reference))
  (|CallParentFunction OtherActor) ; This node is disabled and will not be called.\nDrag off pins to build functionality.
)

(event EventTick
  (params (DeltaSeconds :type Float%20%28single-precision%29))
  (|CallParentFunction DeltaSeconds)
  (if (Variables|Default|GetisDestroying)
    (Actor|DestroyActor)
    (else
      (if (Variables|Default|GetisDeflecting)
        (Variables|Default|Setspeed (Variables|Default|GetnegativeSpeed)))
      (Class|Actor|AddActorWorldTransform (Math|Conversions|ToTransform(Vector) (* (Transformation|GetActorForwardVector) (Variables|Default|GetSpeed))) false false)
      (if (>= 0.0 8.0)
        (Actor|DestroyActor)))))

(fn ConstructionScript
  (|CallParentFunction))

(fn SetMixedAttack
  (Rendering|Material|SetMaterial (Variables|Default|GetStaticMeshComponent) 0 "/Game/StarterContent/Materials/M_Ground_Grass.M_Ground_Grass"))

(fn SetLeftAttack
  (Rendering|Material|SetMaterial (Variables|Default|GetStaticMeshComponent) 0 "/Game/StarterContent/Materials/M_Metal_Steel.M_Metal_Steel"))

(fn SetRightAttack
  (Rendering|Material|SetMaterial (Variables|Default|GetStaticMeshComponent) 0 "/Game/StarterContent/Materials/M_Metal_Gold.M_Metal_Gold"))

(fn DeflectorDestroy
  (params (Impact%20Location :type Vector :default "0, 0, 0") (isLeftHit :type Boolean))
  (|CallParentFunction Impact%20Location isLeftHit)
  (if (Variables|Default|GetisDestroy)
    (Variables|Default|SetisDestroying true)
    (elif isLeftHit
      (if (Utilities|Enum|NotEqual(Enum) (Variables|Default|GetattackType) "NewEnumerator1")
        (Variables|Default|SetisDeflecting true :!label _label)
        (else
          (bind _asvrpawn (Utilities|Casting|CastToVRPawn (Game|Player|GetPlayerPawn 0) :!label _label_2))
          (Default|Hit _asvrpawn)
          (Variables|Default|SetisDestroying true)))
      (elif (Utilities|Enum|NotEqual(Enum) (Variables|Default|GetattackType) "NewEnumerator0")
        (goto _label)
        (else
          (goto _label_2))))))