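; BP_HeadCollider is an invisible collider that stands in for the VR player's head to detect hits.
; Each tick it moves to the VRPawn's HeadPos plus a fixed offset, without following head rotation.
; When its Box overlaps a BP_DeflectOrDestroy actor, it destroys that actor and calls Hit on the VRPawn.
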(event OnComponentBeginOverlap(Box)
  (params (OverlappedComponent :type Primitive%20Component%20Object%20Reference) (OtherActor :type Actor%20Object%20Reference) (OtherComp :type Primitive%20Component%20Object%20Reference) (OtherBodyIndex :type Integer) (bFromSweep :type Boolean) (SweepResult :type Hit%20Result%20Structure%20%28by%20ref%29))
  (bind _asbp_deflect_or_destroy (Utilities|Casting|CastToBP_DeflectOrDestroy OtherActor))
  (Utilities|IsValid _asbp_deflect_or_destroy
    (:Is%20Valid
      (Actor|DestroyActor OtherActor)
      (bind _asvrpawn (Utilities|Casting|CastToVRPawn (Game|Player|GetPlayerPawn 0)))
      (Default|Hit _asvrpawn))))

(event EventBeginPlay
  (Rendering|SetVisibility (Variables|Debug|GetStaticMeshComponent) false false))

(event Collision|EventActorBeginOverlap
  (params (OtherActor :type Actor%20Object%20Reference)))

(event EventTick
  (params (DeltaSeconds :type Float%20%28single-precision%29))
  (bind _asvrpawn (Utilities|Casting|CastToVRPawn (Game|Player|GetPlayerPawn 0)))
  (Utilities|IsValid _asvrpawn
    (:Is%20Valid
      (Transformation|SetActorLocationAndRotation (+ (Variables|/Game/VRTemplate/Blueprints/VRPawn.VRPawn_C|GetHeadPos _asvrpawn) "0.000000,-80.000000,-100.000000") (Math|Rotator|MakeRotator 0.0 0.0 0.0)))))

(fn ConstructionScript)