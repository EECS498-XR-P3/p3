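; BP_DodgeSensor is a sensor actor that counts overlaps with dodge attacks and shows the total on the score display.
; On BeginPlay it finds the BP_Score actor and caches the WBP_ScoreCount widget from that actor's WidgetComponent.
; Each begin overlap with a BP_Dodge_Attack or subclass increments HitCount and pushes it to the widget through SetCount.
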(event EventBeginPlay
  (bind _returnvalue (Actor|GetActorOfClass "/Game/Blueprint/UI/BP_Score.BP_Score_C"))
  (bind _aswbp_score_count (Utilities|Casting|CastToWBP_ScoreCount (UserInterface|GetUserWidgetObject (Actor|GetComponentbyClass _returnvalue "/Script/UMG.WidgetComponent"))))
  (Variables|Default|SetScoreComponent _aswbp_score_count))

(event Collision|EventActorBeginOverlap
  (params (OtherActor :type Actor%20Object%20Reference))
  (if (Utilities|ClassIsChildOf (Utilities|GetClass OtherActor) "/Game/Blueprint/BP_Dodge_Attack.BP_Dodge_Attack_C")
    (bind _output_get (Variables|Default|SetHitCount (+ (Variables|Default|GetHitCount) 1)))
    (Default|SetCount (Variables|Default|GetScoreComponent) _output_get)))

(event EventTick
  (params (DeltaSeconds :type Float%20%28single-precision%29)))

(fn ConstructionScript)