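; Jab attack actor that travels along its forward vector as a moving attack and can be deflected.
; BeginPlay caches a negated Speed, which Tick swaps in while IsDeflecting is set to reverse the direction.
; Tick moves the actor without sweep by a per-frame step that ignores delta time.
; Its DestroyActor check compares two constants, so it never fires.
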(event EventBeginPlay
  (|CallParentFunction)
  (Variables|Default|SetnegativeSpeed (* (Variables|Default|Getspeed) -1.0)))

(event Collision|EventActorBeginOverlap
  (params (OtherActor :type Actor%20Object%20Reference))
  (|CallParentFunction OtherActor) ; This node is disabled and will not be called.\nDrag off pins to build functionality.
)

(event EventTick
  (params (DeltaSeconds :type Float%20%28single-precision%29))
  (|CallParentFunction DeltaSeconds)
  (if (Variables|Default|GetisDeflecting)
    (Variables|Default|Setspeed (Variables|Default|GetnegativeSpeed)))
  (Class|Actor|AddActorWorldTransform (Math|Conversions|ToTransform(Vector) (* (Transformation|GetActorForwardVector) (Variables|Default|GetSpeed))) false false)
  (if (>= 0.0 8.0)
    (Actor|DestroyActor)))

(fn ConstructionScript
  (|CallParentFunction))